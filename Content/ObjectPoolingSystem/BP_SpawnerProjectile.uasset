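; Test spawner actor that fires pooled projectiles along its forward vector.
; BeginPlay creates an object pool for the projectile class and prints two keyed debug messages separated by a delay.
; Every Tick, without throttling, it takes a projectile from the pool and activates it just ahead of the actor, passing transform plus Name, ID and Text data.
; Leftover unconnected nodes experiment with string, name and text functions.
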(event EventBeginPlay
  (CallFunction|CreateObjectPool (Variables|Default|GetProjectileClass))
  (Development|PrintString "HELLO IN BLU" true true "(R=0.000000,G=0.660000,B=1.000000,A=1.000000)" 5.0 "NameExample")
  (Utilities|FlowControl|Delay 2.0)
  (Development|PrintString "HELLO IN ROSSO" true true "(R=1.000000,G=0.000000,B=0.083632,A=1.000000)" 5.0 "nameexample"))

(event Collision|EventActorBeginOverlap
  (params (OtherActor :type Actor%20Object%20Reference)))

(event EventTick
  (params (DeltaSeconds :type Float%20%28single-precision%29))
  (bind _returnvalue (Transformation|GetActorForwardVector))
  (bind _objectpoolref (CallFunction|GetProjectilefromPool (Variables|Default|GetProjectileClass)))
  (bind _output_get (Variables|Default|SetObject%20Pool%20Activation%20Data (Utilities|Struct|MakeObjectPoolActivationData (Math|Transform|MakeTransform (+ (Transformation|GetActorLocation) (* _returnvalue 1e+02)) (Math|Rotator|MakeRotfromX _returnvalue) "1.000000,1.000000,1.000000") (Variables|Default|GetObject%20Pool%20Name) (Variables|Default|GetObject%20Pool%20ID) (Variables|Default|GetObject%20Pool%20Text))))
  (Class|ObjectPoolInterface|Activate _objectpoolref _output_get))

(fn ConstructionScript)